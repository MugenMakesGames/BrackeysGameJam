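; Player pawn that lets the player snap its view between forward, left and right with smooth camera turns.
; Enhanced Input actions drive one timeline per side, which sets the PlayerView yaw on update.
; Left and right turns start only from exactly forward, and turning forward reverses the timeline of whichever side the view currently faces.
; Exact world-rotation checks act as the state, so turn requests made mid-turn are ignored.
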(event Input|EnhancedActionEvents|EnhancedInputActionIA_ChooseTopic
  (params (ActionValue :type Boolean) (ElapsedSeconds :type Float%20%28double-precision%29) (TriggeredSeconds :type Float%20%28double-precision%29) (InputAction :type Input%20Action%20Object%20Reference :default "/Game/My_Content/Input/Actions/IA_ChooseTopic.IA_ChooseTopic")))

(event Input|EnhancedActionEvents|EnhancedInputActionIA_TurnForward
  (params (ActionValue :type Boolean) (ElapsedSeconds :type Float%20%28double-precision%29) (TriggeredSeconds :type Float%20%28double-precision%29) (InputAction :type Input%20Action%20Object%20Reference :default "/Game/My_Content/Input/Actions/IA_TurnForward.IA_TurnForward"))
  ;[0.07619 0.15 0.05951 0.502] Check if the camera is rotated to the right or left before rotating forward
  (:Started
    (Utilities|FlowControl|Sequence
      (:then_0
        (if (Utilities|Operators|EqualEqual (Transformation|GetWorldRotation (Variables|Default|GetPlayerView)) "0.000000,-90.000000,0.000000" 0.0)
          ;[0.07548 0.15 0.0592 0.5] Smooth turn animation (Left)
          (bind _turncamera__left_ (Timeline|Turn%20Camera%20%28Left%29 ReverseFromEnd)
            (:Update
              (Transformation|SetWorldRotation (Variables|Default|GetPlayerView) (Math|Rotator|MakeRotator 0.0 0.0 _turncamera__left_) false false)))))
      (:then_1
        (if (Utilities|Operators|EqualEqual (Transformation|GetWorldRotation (Variables|Default|GetPlayerView)) "0.000000,90.000000,0.000000" 0.0)
          ;[0.07619 0.15 0.05951 0.502] Smooth turn animation (Right)
          (bind _turncamera__right_ (Timeline|Timeline ReverseFromEnd)
            (:Update
              (Transformation|SetWorldRotation (Variables|Default|GetPlayerView) (Math|Rotator|MakeRotator 0.0 0.0 _turncamera__right_) false false))))))))

(event Input|EnhancedActionEvents|EnhancedInputActionIA_TurnRight
  (params (ActionValue :type Boolean) (ElapsedSeconds :type Float%20%28double-precision%29) (TriggeredSeconds :type Float%20%28double-precision%29) (InputAction :type Input%20Action%20Object%20Reference :default "/Game/My_Content/Input/Actions/IA_TurnRight.IA_TurnRight"))
  ;[0.07619 0.15 0.05951 0.502] Smooth turn animation (Right)
  (:Started
    (if (Utilities|Operators|EqualEqual (Transformation|GetWorldRotation (Variables|Default|GetPlayerView)) "0.000000,0.000000,0.000000" 0.0)
      (bind _turncamera__right_ (Timeline|Timeline Play)
        (:Update
          (Transformation|SetWorldRotation (Variables|Default|GetPlayerView) (Math|Rotator|MakeRotator 0.0 0.0 _turncamera__right_) false false))))))

(event Input|EnhancedActionEvents|EnhancedInputActionIA_TurnLeft
  (params (ActionValue :type Boolean) (ElapsedSeconds :type Float%20%28double-precision%29) (TriggeredSeconds :type Float%20%28double-precision%29) (InputAction :type Input%20Action%20Object%20Reference :default "/Game/My_Content/Input/Actions/IA_TurnLeft.IA_TurnLeft"))
  ;[0.07548 0.15 0.0592 0.5] Smooth turn animation (Left)
  (:Started
    (if (Utilities|Operators|EqualEqual (Transformation|GetWorldRotation (Variables|Default|GetPlayerView)) "0.000000,0.000000,0.000000" 0.0)
      (bind _turncamera__left_ (Timeline|Turn%20Camera%20%28Left%29 Play)
        (:Update
          (Transformation|SetWorldRotation (Variables|Default|GetPlayerView) (Math|Rotator|MakeRotator 0.0 0.0 _turncamera__left_) false false))))))

(event Collision|EventActorBeginOverlap
  (params (OtherActor :type Actor%20Object%20Reference)))

(event EventTick
  (params (DeltaSeconds :type Float%20%28single-precision%29)))

(event EventBeginPlay
  ;[0.15 0.15 0.15 0.5] Getting player start rotation
)

(fn ConstructionScript)